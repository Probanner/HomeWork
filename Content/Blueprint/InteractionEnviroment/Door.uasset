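; Automatic door Blueprint that opens and closes as the player character class BP_Character moves through its trigger boxes.
; Beginning an overlap with EnterBox calls Opening, and beginning one with ExitBox calls Closing, with IsDoorOpen blocking repeat triggers.
; One timeline plays forward or in reverse, its ZOffset remapped through a clamped range to slide the Door vertically by the Z variable.
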(event `self.EnterBox.OnComponentBeginOverlap`
  (params (OverlappedComponent :type "PrimitiveComponent Object Reference") (OtherActor :type "Actor Object Reference") (OtherComp :type "PrimitiveComponent Object Reference") (OtherBodyIndex :type Integer) (bFromSweep :type Boolean) (SweepResult :type "HitResult Structure (by ref)"))
  (cast `/Game/Blueprint/Characters/BP_Character` OtherActor)
  (`self.Opening`))

(event `self.ExitBox.OnComponentBeginOverlap`
  (params (OverlappedComponent :type "PrimitiveComponent Object Reference") (OtherActor :type "Actor Object Reference") (OtherComp :type "PrimitiveComponent Object Reference") (OtherBodyIndex :type Integer) (bFromSweep :type Boolean) (SweepResult :type "HitResult Structure (by ref)"))
  (cast `/Game/Blueprint/Characters/BP_Character` OtherActor)
  (`self.Closing`))

(event `Closing`
  (if (`self.bIsDoorOpen`)
    (set `self.bIsDoorOpen` false)
    (bind (_direction _zoffset) (`Timeline|DoorOpenClose` :!via `ReverseFromEnd` :!label _label)
      (:`Update`
        (`SceneComponent.K2_SetRelativeLocation` (`self.Door`) (`KismetMathLibrary.MakeVector` 0.0 0.0 (`KismetMathLibrary.MapRangeClamped` _zoffset 0.0 1.0 0.0 (`self.Z`))) false false)))))

(event `Opening`
  (if (not (`self.bIsDoorOpen`))
    (set `self.bIsDoorOpen` true)
    (goto _label :!via `PlayFromStart`)))

(fn `UserConstructionScript`)
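; Lobby game mode that tracks connected players, shares the selected level with them and launches the game.
; PostLogin and OnLogout maintain the list of BP_LobbyPlayerControllers, and each new one receives the current level choice.
; UpdateLevelName stores a new selection and refreshes each client's lobby widget.
; LaunchGame clears players' widgets, then runs a servertravel console command built from the selected level; SaveColorForPlayers is an empty stub.
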(event `LaunchGame`
  (for _array_element (`self.PlayerControllers`)
    (bind _asbp_lobby_player_controller (cast `/Game/Blueprint/Game/Lobby/BP_LobbyPlayerController` _array_element))
    (`/Game/Blueprint/Game/Lobby/BP_LobbyPlayerController.RemoveAllWidgets` _asbp_lobby_player_controller))
  (`KismetSystemLibrary.ExecuteConsoleCommand` (`KismetStringLibrary.Concat_StrStr` "servertravel " (`KismetStringLibrary.Conv_NameToString` (`self.SelectedLevel`))) (`GameplayStatics.GetPlayerController` 0)))

(event `SaveColorForPlayers`)

(event `UpdateLevelName`
  (params (SelectedLevel :type Name))
  (set `self.SelectedLevel` SelectedLevel)
  (for _array_element (`self.PlayerControllers`)
    (bind _asbp_lobby_player_controller (cast `/Game/Blueprint/Game/Lobby/BP_LobbyPlayerController` _array_element))
    (`/Game/Blueprint/Game/Lobby/BP_LobbyPlayerController.UpdateLobbyWidgetOnClient` _asbp_lobby_player_controller (`self.SelectedLevel`))))

(event `self.K2_PostLogin`
  (params (NewPlayer :type "PlayerController Object Reference"))
  (bind _asbp_lobby_player_controller (cast `/Game/Blueprint/Game/Lobby/BP_LobbyPlayerController` NewPlayer))
  (`KismetArrayLibrary.Array_Add` (`self.PlayerControllers`) _asbp_lobby_player_controller)
  (set `/Game/Blueprint/Game/Lobby/BP_LobbyPlayerController.CurrentLevelByHost` (`self.SelectedLevel`) _asbp_lobby_player_controller))

(event `self.K2_OnLogout`
  (params (ExitingController :type "Controller Object Reference"))
  (bind _asbp_lobby_player_controller (cast `/Game/Blueprint/Game/Lobby/BP_LobbyPlayerController` ExitingController))
  (`KismetArrayLibrary.Array_RemoveItem` (`self.PlayerControllers`) _asbp_lobby_player_controller))

(fn `UserConstructionScript`)
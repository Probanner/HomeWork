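; Lobby player controller that shows the lobby menu with a mouse cursor over a level camera view for the local player.
; On the host, it fills the menu with level buttons from DT_Levels and reports the first level to BP_LobbyMode as the default.
; Clients display the host's current level, and events update the shown level and player name or clear widgets.
; UpdateMeReady is an empty stub.
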(event `self.ReceiveBeginPlay`
  (bind _returnvalue (`KismetSystemLibrary.IsServer`))
  (bind _lobbymenu (`self.LobbyMenu`))
  (if (`self.IsLocalController`)
    (set `self.bShowMouseCursor` true)
    (bind _returnvalue_2 (`GameplayStatics.GetActorOfClass` "/Script/Engine.CameraActor"))
    (`self.SetViewTargetWithBlend` _returnvalue_2)
    (bind _returnvalue_3 (`|CreateWidget` "/Game/Widget/LobbyMenu/BPW_LobbyMenu.BPW_LobbyMenu_C" null _returnvalue "" (`KismetStringLibrary.Conv_NameToString` (`self.CurrentLevelByHost`))))
    (bind _output_get (set `self.LobbyMenu` _returnvalue_3))
    (`UserWidget.AddToViewport` _output_get 0)
    (if _returnvalue
      (bind _outrownames (`DataTableFunctionLibrary.GetDataTableRowNames` "/Game/Table/Levels/DT_Levels.DT_Levels"))
      (bind _returnvalue_4 (`|GetDataTableRow` "/Game/Table/Levels/DT_Levels.DT_Levels" (`|GetArrayItem` _outrownames))
        (:`then`
          (bind _levelname (break `/Game/Table/Levels/F_Levels` _returnvalue_4))
          (`/Game/Widget/LobbyMenu/BPW_LobbyMenu.UpdateLevelName` (`self.LobbyMenu`) _levelname)
          (`self.UpdatePlayerSelectedMap` _levelname)
          (for _array_element _outrownames
            (bind _returnvalue_5 (`|GetDataTableRow` "/Game/Table/Levels/DT_Levels.DT_Levels" _array_element)
              (:`then`
                (bind _returnvalue_6 (`|CreateWidget` "/Game/Widget/LobbyMenu/BP_LobbyLevelButton.BP_LobbyLevelButton_C" null (`.LevelName_2_A0B6B0DC42B989B88316D6AA02E00B2D` (break `/Game/Table/Levels/F_Levels` _returnvalue_5)) _lobbymenu))
                (`VerticalBox.AddChildToVerticalBox` (`/Game/Widget/LobbyMenu/BPW_LobbyMenu.SelectlvlByHost_Box` _lobbymenu) _returnvalue_6))
              (:`RowNotFound`
                (`KismetSystemLibrary.PrintString` "No Level founded!" true true (struct :`R` 1.0 :`A` 1.0) :!label _label)))))
        (:`RowNotFound`
          (goto _label)))
      (else
        (`/Game/Widget/LobbyMenu/BPW_LobbyMenu.UpdateLevelName` (`self.LobbyMenu`) (`self.CurrentLevelByHost`))))))

(event `UpdateMeReady`)

(event `UpdatePlayerSelectedMap`
  (params (CurrentLevelByServer :type Name))
  (bind _asbp_lobby_mode (cast `/Game/Blueprint/Game/Lobby/BP_LobbyMode` (`GameplayStatics.GetGameMode`)))
  (`/Game/Blueprint/Game/Lobby/BP_LobbyMode.UpdateLevelName` _asbp_lobby_mode CurrentLevelByServer))

(event `UpdateLobbyWidgetOnClient`
  (params (SelectedLevel :type Name))
  (`/Game/Widget/LobbyMenu/BPW_LobbyMenu.UpdateLevelName` (`self.LobbyMenu`) SelectedLevel))

(event `UpdatePlayerName`
  (params (PlayerName :type Text))
  (`TextBlock.SetText` (`/Game/Widget/LobbyMenu/BPW_LobbyMenu.PlayerName` (`self.LobbyMenu`)) PlayerName))

(event `RemoveAllWidgets`
  (`WidgetLayoutLibrary.RemoveAllWidgets`))

(fn `UserConstructionScript`)
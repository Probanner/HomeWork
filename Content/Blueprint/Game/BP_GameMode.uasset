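; BP_GameMode is the game mode that handles phase-based player spawning and score forwarding.
; Initial spawns use the player start tagged Phase1.
; TryToRespawn asks BP_GameState whether respawn is allowed, then restarts the player at the start matching the current phase (Phase1 to Phase3) and returns the result.
; SaveScore passes score changes to the game state.
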(fn `ChoosePlayerStart`
  (params (Player :type "Controller Object Reference"))
  (returns (ReturnValue :type "Actor Object Reference"))
  (return (`self.K2_FindPlayerStart` Player "Phase1")))

(fn `SaveScore`
  (params (Score :type Integer))
  (bind _asbp_game_state (cast `/Game/Blueprint/Game/BP_GameState` (`GameplayStatics.GetGameState`)))
  (`/Game/Blueprint/Game/BP_GameState.ChangeScore` _asbp_game_state Score))

(fn `TryToRespawn`
  (params (PlayerController :type "PlayerController Object Reference"))
  (returns (Success :type Boolean))
  (bind _asbp_game_state (cast `/Game/Blueprint/Game/BP_GameState` (`GameplayStatics.GetGameState`)))
  (bind (_success _currentphase) (`/Game/Blueprint/Game/BP_GameState.Can Player Respawn` _asbp_game_state))
  (if _success
    (`self.RestartPlayerAtPlayerStart` PlayerController (`self.K2_FindPlayerStart` null (select `/Game/Blueprint/CheckPoint/E_Phases` _currentphase :`NewEnumerator0` "Phase1" :`NewEnumerator1` "Phase2" :`NewEnumerator2` "Phase3")))
    (return true)
    (else
      (return _success))))

(fn `UserConstructionScript`)
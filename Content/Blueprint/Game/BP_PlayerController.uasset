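; Player controller Blueprint that manages the lifetime of the in-game UI widget.
; Possess calls CreateWidgets unless IsOnBeginPlay is set, and UnPossess removes the stored widget from its parent.
; CreateWidgets branches on authority, adding the widget for a local controller on authority or directly on remote.
; BeginPlay and Tick are empty, and leftover unconnected nodes include a weapon-reload debug widget.
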(event `self.ReceiveBeginPlay`)

(event `self.ReceiveTick`
  (params (DeltaSeconds :type "Float (single-precision)")))

(event `self.ReceiveUnPossess`
  (params (UnpossessedPawn :type "Pawn Object Reference"))
  (bind _ingamewidgetref (`self.IngameWidgetRef`))
  (`/Engine/EditorBlueprintResources/StandardMacros.IsValid` _ingamewidgetref
    (:`Is Valid`
      (`Widget.RemoveFromParent` _ingamewidgetref))))

(event `self.ReceivePossess`
  (params (PossessedPawn :type "Pawn Object Reference"))
  (if (not (`self.bIsOnBeginPlay`))
    (`self.CreateWidgets`)))

(fn `CreateWidgets`
  (`/Engine/EditorBlueprintResources/ActorMacros.Switch Has Authority`
    (:`Authority`
      (if (`self.IsLocalPlayerController`)
        (bind _returnvalue (`|CreateWidget` "/Game/Widget/InGameWidget.InGameWidget_C" self :!label _label))
        (set `self.IngameWidgetRef` _returnvalue)
        (`UserWidget.AddToViewport` _returnvalue 0)))
    (:`Remote`
      (goto _label))))

(fn `UserConstructionScript`)
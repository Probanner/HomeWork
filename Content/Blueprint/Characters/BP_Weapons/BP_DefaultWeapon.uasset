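; BP_DefaultWeapon is a weapon Blueprint with a helper for spawning projectile actors.
; SpawnProjectileFunc spawns the given class, passing timing, lifespan, projectile info, spawn location and brush material.
; The ProjectileRespawn event is empty: its disconnected logic would lazily create and cache a dynamic brush material from the weapon's skeletal brush setting, then call that helper.
; BeginPlay and the construction script are also empty.
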(event `self.ReceiveBeginPlay`)

(event `self.ProjectileRespawn`
  (params (_ProjectileToRespawn :type "DefaultProjectile Class Reference") (_initialSpeed :type "Float (single-precision)") (_SpawnLocation :type "Vector Structure") (_SpawnRotation :type "Rotator Structure") (_SpanLifeTime :type "Float (single-precision)") (_ProjectileInfo :type "ProjectileInfo Structure")))

(fn `SpawnProjectileFunc`
  (params (Class :type "/Game/Blueprint/Characters/BP_Projectiles/BP_DefaultProjectile Class Reference") (InitialTime :type "Float (double-precision)") (SpawnTransform :type "Transform Structure") (SpanLifeTime :type "Float (double-precision)") (ProjectileInfo :type "ProjectileInfo Structure") (SpawnLocation :type "Vector Structure") (SkeletalBrush :type "MaterialInstanceDynamic Object Reference"))
  (`|SpawnActorFromClass` Class SpawnTransform "Undefined" "OverrideRootScale" null InitialTime SpanLifeTime ProjectileInfo SpawnLocation SkeletalBrush null))

(fn `UserConstructionScript`)
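; Default projectile Blueprint that paints damage onto skeletal meshes at the UV it hits.
; Its RenderTargetPrint event receives the hit UV, offsets a brush material to it and draws that into the target actor's render target.
; On an actor's first hit, it creates that render target, caches it in BP_GameState by display name and binds it as DamageTexture through new dynamic material instances.
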(event `self.ReceiveBeginPlay`)

(event `RenderTargetPrint_1`
  (params (HitComp :type "PrimitiveComponent Object Reference") (OtherActor :type "Actor Object Reference") (OtherComponent :type "PrimitiveComponent Object Reference") (NormalImpulse :type "Vector Structure") (Hit :type "HitResult Structure (by ref)") (HittedUV :type "Vector2D Structure"))
  (bind _asskeletal_mesh_component (cast `SkeletalMeshComponent` (`.HitComponent` (`GameplayStatics.BreakHitResult` Hit))))
  (`self.Print on Skeletal Mesh` OtherActor _asskeletal_mesh_component (struct) HittedUV))

(fn `Print on Skeletal Mesh`
  (params (OtherActor :type "Actor Object Reference") (OtherComponent :type "PrimitiveComponent Object Reference") (Hit :type "HitResult Structure") (UVHitted :type "Vector2D Structure"))
  (bind _returnvalue (`KismetSystemLibrary.GetDisplayName` OtherActor))
  (bind _brush (`self.Brush`))
  (bind _brush_2 (`self.Brush`))
  (`KismetSystemLibrary.PrintString` (`KismetStringLibrary.Conv_Vector2dToString` UVHitted))
  (`/Engine/EditorBlueprintResources/StandardMacros.IsValid` (`self.Brush`)
    (:`Is Valid`
      (bind _asbp_game_state (cast `/Game/Blueprint/Game/BP_GameState` (`GameplayStatics.GetGameState`)))
      (bind _asskeletal_mesh_component (cast `SkeletalMeshComponent` OtherComponent))
      (bind _mapnametort (`/Game/Blueprint/Game/BP_GameState.MapNameToRT` _asbp_game_state))
      (if (`BlueprintMapLibrary.Map_Contains` _mapnametort _returnvalue)
        (`MaterialInstanceDynamic.SetVectorParameterValue` _brush "Offset" (`KismetMathLibrary.Conv_VectorToLinearColor` (`KismetMathLibrary.Conv_Vector2DToVector` UVHitted)))
        (`KismetRenderingLibrary.DrawMaterialToRenderTarget` (`BlueprintMapLibrary.Map_Find` _mapnametort _returnvalue) _brush)
        (else
          (bind _returnvalue_2 (`KismetRenderingLibrary.CreateRenderTarget2D` 1024 1024))
          (bind _output_get (set `self.CreatedRendetTarget` _returnvalue_2))
          (`BlueprintMapLibrary.Map_Add` _mapnametort _returnvalue _output_get)
          (for (_array_element _array_index) (`MeshComponent.GetMaterials` _asskeletal_mesh_component)
            (bind _returnvalue_3 (`KismetMaterialLibrary.CreateDynamicMaterialInstance` _array_element))
            (`KismetArrayLibrary.Array_Add` (`self.MaterialInstanceArray`) _returnvalue_3)
            (`PrimitiveComponent.SetMaterial` _asskeletal_mesh_component _array_index _returnvalue_3)
            (`MaterialInstanceDynamic.SetTextureParameterValue` _returnvalue_3 "DamageTexture" (`self.CreatedRendetTarget`)))
          (`MaterialInstanceDynamic.SetVectorParameterValue` _brush_2 "Offset" (`KismetMathLibrary.Conv_VectorToLinearColor` (`KismetMathLibrary.Conv_Vector2DToVector` UVHitted)))
          (`KismetRenderingLibrary.DrawMaterialToRenderTarget` (`self.CreatedRendetTarget`) _brush_2))))))

(fn `UserConstructionScript`)
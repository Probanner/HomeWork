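; BP_LowArmor is a low-tier armor pickup that restores a character's shield, built on a parent item class.
; On TakingItem, if the shield is below 100, it adds ShieldValue through the character's health component, plays a sound and destroys itself.
; BeginPlay enables custom depth and stencil on the mesh and particle system.
; Tick spins the root by a fixed step each frame, independent of delta time.
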(event `self.ReceiveBeginPlay`
  (`parent.ReceiveBeginPlay`)
  (`PrimitiveComponent.SetRenderCustomDepth` (`self.ParticleSystem`) true)
  (`PrimitiveComponent.SetRenderCustomDepth` (`self.StaticMesh`) true)
  (`PrimitiveComponent.SetCustomDepthStencilValue` (`self.StaticMesh`) 1)
  (`PrimitiveComponent.SetCustomDepthStencilValue` (`self.ParticleSystem`) 1))

(event `self.ReceiveActorBeginOverlap`
  (params (OtherActor :type "Actor Object Reference"))
  (`parent.ReceiveActorBeginOverlap` OtherActor))

(event `self.ReceiveTick`
  (params (DeltaSeconds :type "Float (single-precision)"))
  (bind _defaultsceneroot (`self.DefaultSceneRoot`))
  (`parent.ReceiveTick` DeltaSeconds)
  (`/Engine/EditorBlueprintResources/StandardMacros.IsValid` _defaultsceneroot
    (:`Is Valid`
      (`SceneComponent.K2_AddRelativeRotation` _defaultsceneroot (struct :`Yaw` 1.0) false false))))

(event `self.TakingItem`
  (params (CharHealthComponent :type "CharHealthComponent Object Reference"))
  (bind _returnvalue (`CharHealthComponent.GetCurrentShield` CharHealthComponent))
  (if (< _returnvalue 100.0)
    (`CharHealthComponent.ChangeShieldValue` CharHealthComponent (`self.ShieldValue`))
    (`GameplayStatics.PlaySound2D` "/Game/Blueprint/Characters/BuffItems/FirstAidKit/HealSound.HealSound" 1.0 1.0 0.0 null null)
    (`self.K2_DestroyActor`)))

(fn `UserConstructionScript`
  (`parent.UserConstructionScript`))
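; BP_FirstAidKit is a rotating health pickup that heals a BP_Character on overlap.
; The overlap passes the character's health component to TakingItem, which adds HealthValue only if current health is below a hard-coded 100.
; A successful pickup plays a 2D heal sound through SpawnSoundOnClient, then destroys the actor.
; BeginPlay enables custom depth and stencil on the mesh and particle system.
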(event `self.ReceiveBeginPlay`
  (`parent.ReceiveBeginPlay`)
  (`PrimitiveComponent.SetRenderCustomDepth` (`self.ParticleSystem`) true)
  (`PrimitiveComponent.SetRenderCustomDepth` (`self.StaticMesh`) true)
  (`PrimitiveComponent.SetCustomDepthStencilValue` (`self.StaticMesh`) 1)
  (`PrimitiveComponent.SetCustomDepthStencilValue` (`self.ParticleSystem`) 1))

(event `self.ReceiveTick`
  (params (DeltaSeconds :type "Float (single-precision)"))
  (`parent.ReceiveTick` DeltaSeconds)
  (`SceneComponent.K2_AddRelativeRotation` (`self.DefaultSceneRoot`) (struct :`Yaw` 1.0) false false))

(event `self.TakingItem`
  (params (CharHealthComponent :type "CharHealthComponent Object Reference"))
  (bind _returnvalue (`HeathComponent.GetCurrentHealth` CharHealthComponent))
  (if (< _returnvalue 100.0)
    (`HeathComponent.ChangeCurrentHealth` CharHealthComponent (`self.HealthValue`))
    (`self.SpawnSoundOnClient`)
    (`self.K2_DestroyActor`)))

(event `self.ReceiveActorBeginOverlap`
  (params (OtherActor :type "Actor Object Reference"))
  (bind _asbp_character (cast `/Game/Blueprint/Characters/BP_Character` OtherActor))
  (`self.TakingItem` (`HomeWork22Character.CharHealthComp` _asbp_character)))

(event `SpawnSoundOnClient`
  (`GameplayStatics.PlaySound2D` "/Game/Blueprint/Characters/BuffItems/FirstAidKit/HealSound.HealSound" 1.0 1.0 0.0 null null))

(fn `UserConstructionScript`
  (`parent.UserConstructionScript`))
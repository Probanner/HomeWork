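; Top-down player character for a networked shooter, handling weapon inventory, pickups, loot cases and death.
; BeginPlay seeds WeaponSwitchComponent from the GameInstance; dropped weapons spawn as physics-launched pickups.
; Net events show swap and loot widgets only on the locally controlled pawn, while other events spawn damage numbers and the death screen.
; Camera functions provide shake, instant or timer-stepped boom zoom, and trace-to-cursor material swapping on blocking SM_L actors.
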(event `self.ReceiveTick`
  (params (DeltaSeconds :type "Float (single-precision)")))

(event `self.ReceiveBeginPlay`
  ;[1 1 1] Begin Play
  (bind _asbp_game_instance (cast `/Game/Blueprint/Game/BP_GameInstance` (`GameplayStatics.GetGameInstance`)))
  (`WeaponSwitchActor.InitInventory_OnServer` (`self.WeaponSwitchComponent`) (`/Game/Blueprint/Game/BP_GameInstance.WeaponSlotGI` _asbp_game_instance) (`/Game/Blueprint/Game/BP_GameInstance.AmmoSlotGI` _asbp_game_instance))
  (`WeaponSwitchActor.SwitchWeaponToIndex` (`self.WeaponSwitchComponent`) 0)
  (`/Engine/EditorBlueprintResources/ActorMacros.Switch Has Authority`
    (:`Authority`
      (`KismetSystemLibrary.Delay` 2.0))
    (:`Remote`
      _))
  (bind _asbp_player_controller (cast `/Game/Blueprint/Game/BP_PlayerController` (`GameplayStatics.GetPlayerController` 0))
    (:`then`
      (`/Game/Blueprint/Game/BP_PlayerController.CreateWidgets` _asbp_player_controller))
    (:`CastFailed`
      (`KismetSystemLibrary.PrintString` "FAIL" true true (struct :`G` 0.66 :`B` 1.0 :`A` 1.0) 30.0))))

(event `self.SpawnDamageWidget`
  (params (CurrentHealth :type "Float (single-precision)") (Damage :type "Float (single-precision)"))
  ;[1 1 1] DamageWidget
  (bind _returnvalue (`|SpawnActorFromClass` "/Game/Blueprint/Characters/CanTakeDamageObjects/DisplayDamageActor.DisplayDamageActor_C" (`KismetMathLibrary.MakeTransform` (+ (`self.K2_GetActorLocation`) (+ (`self.LocalPointSpawnHealthNumber`) (`KismetMathLibrary.MakeVector` (`KismetMathLibrary.RandomFloatInRange` 0.0 40.0) (`KismetMathLibrary.RandomFloatInRange` 0.0 40.0))))) "Undefined" "OverrideRootScale" null null))
  (`/Game/Blueprint/Characters/CanTakeDamageObjects/DisplayDamageActor.InitActor` _returnvalue Damage CurrentHealth))

(event `NoSpaceEvent`
  (params (NewWeapon :type "/Game/Blueprint/Characters/PickUpWeapons/PickupActor_Weapon Object Reference"))
  (`self.StartSwitchWeapon_OnClient` NewWeapon))

(event `StartSwitchWeapon_OnClient`
  (params (NewWeapon :type "/Game/Blueprint/Characters/PickUpWeapons/PickupActor_Weapon Object Reference"))
  ;[1 1 1] Weapon From Floor
  (if (`self.IsLocallyControlled`)
    (bind _returnvalue (`|CreateWidget` "/Game/Widget/Inventory/SwitchWeaponWidget.SwitchWeaponWidget_C"))
    (`UserWidget.AddToViewport` _returnvalue 0)
    (set `self.PickupedWeapon` NewWeapon)))

(event `EndSwitchWeaponEvent`
  ;[1 1 1] Weapon From Floor
  (`self.EndSwitchWeapon_OnClient`))

(event `EndSwitchWeapon_OnClient`
  ;[1 1 1] Weapon From Floor
  (if (`self.IsLocallyControlled`)
    (bind _foundwidgets (`WidgetBlueprintLibrary.GetAllWidgetsOfClass` "/Game/Widget/Inventory/SwitchWeaponWidget.SwitchWeaponWidget_C"))
    (for _array_element _foundwidgets
      (`Widget.RemoveFromParent` _array_element)
      (set `self.PickupedWeapon` null))))

(event `self.DropWeaponItem`
  (params (WeaponToDrop :type "DropItem Structure"))
  (bind (_actortodrop _bisaweapon _weaponname) (break `DropItem` WeaponToDrop))
  (bind (_returnvalue_x _returnvalue_y _returnvalue_z) (`KismetMathLibrary.BreakVector` (`self.K2_GetActorLocation`)))
  (bind _aspickup_actor_weapon (castclass `/Game/Blueprint/Characters/PickUpWeapons/PickupActor_Weapon` _actortodrop))
  (bind _returnvalue (`|SpawnActorFromClass` _aspickup_actor_weapon (`KismetMathLibrary.MakeTransform` (+ (* (`KismetMathLibrary.Normal` (`SceneComponent.GetForwardVector` (`self.CapsuleComponent`))) 1.0) (`KismetMathLibrary.MakeVector` _returnvalue_x _returnvalue_y (+ _returnvalue_z 50.0)))) "Undefined" "OverrideRootScale" null WeaponToDrop null))
  (bind _collisionsphere (`PickupActor.CollisionSphere` _returnvalue))
  (`PrimitiveComponent.SetSimulatePhysics` _collisionsphere true)
  (`PrimitiveComponent.AddImpulse` _collisionsphere (* (`KismetMathLibrary.Normal` (`SceneComponent.GetForwardVector` (`self.CapsuleComponent`))) 600.0) "None" true)
  (`self.DropMulticast` _weaponname))

(event `DropMulticast`
  (params (WeaponName :type Name))
  (`self.OnWeaponDropDispatcher` WeaponName))

(event `Key|B`
  (params (Key :type "Key Structure"))
  (:`Pressed`
    (bind _returnvalue (`|CreateWidget` "/Game/Widget/MainMenu/BPW_Option.BPW_Option_C"))
    (`UserWidget.AddToViewport` _returnvalue 0)
    (set `PlayerController.bShowMouseCursor` true (`GameplayStatics.GetPlayerController` 0))))

(event `LootCaseStartOverlap`
  (params (BP_Spawn_Loot :type "/Game/Blueprint/Characters/BP_WeaponSpawners/BP_SpawnLootActor_Default Object Reference"))
  ;[1 1 1] Net Widgets
  (set `self.BP Spawn Loot` BP_Spawn_Loot)
  (`self.NetLootCaseStartOverLapWidget`))

(event `NetLootCaseStartOverLapWidget`
  ;[1 1 1] Net Widgets
  (if (`self.IsLocallyControlled`)
    (bind _returnvalue (`|CreateWidget` "/Game/Widget/Inventory/LootCaseWidget.LootCaseWidget_C"))
    (`UserWidget.AddToViewport` _returnvalue 0)
    (set `self.LootWidget` _returnvalue)))

(event `LootCaseOverlapEnd`
  ;[1 1 1] Net Widgets
  (`self.NetLootCaseOverlapEndWidget`))

(event `NetLootCaseOverlapEndWidget`
  ;[1 1 1] Net Widgets
  (if (`self.IsLocallyControlled`)
    (bind _foundwidgets (`WidgetBlueprintLibrary.GetAllWidgetsOfClass` "/Game/Widget/Inventory/LootCaseWidget.LootCaseWidget_C" false))
    (for _array_element _foundwidgets
      (`Widget.RemoveFromParent` _array_element))
    (set `self.PickupedWeapon` null)
    (set `self.BP Spawn Loot` null)))

(event `Key|F`
  (params (Key :type "Key Structure"))
  (:`Pressed`
    (`/Engine/EditorBlueprintResources/StandardMacros.IsValid` (`self.BP Spawn Loot`)
      (:`Is Valid`
        (`self.F_Multicast`)))))

(event `F_Multicast`
  (`/Game/Blueprint/Characters/BP_WeaponSpawners/BP_SpawnLootActor_Default.Spawn Pickup Actor` (`self.BP Spawn Loot`)))

(event `self.CharDead_BP`
  (`self.CharDead`))

(fn `CameraShakeEvent`
  (`GameplayStatics.PlayWorldCameraShake` "/Game/Blueprint/Game/BP_CameraShake.BP_CameraShake_C" (`SceneComponent.K2_GetComponentLocation` (`self.TopDownCameraComponent`)) 0.0 30.0))

(fn `CameraSmoothZoom`
  (params (A :type "Float (double-precision)"))
  (set `self.SlideDone` false)
  (if (!= A 0.0)
    (if (> A 0.0)
      (set `self.SlideUp` false)
      (else
        (set `self.SlideUp` true)))
    (if (not (`self.SlideDone`))
      (bind _returnvalue (`KismetSystemLibrary.K2_SetTimer` null "CameraTick" (`self.TimerTick`) true))
      (set `self.TimerSlide` _returnvalue))))

(fn `CameraTick`
  (bind _cameraboom (`self.CameraBoom`))
  (bind _cameratickstep (`self.CameraTickStep`))
  (bind _targetarmlength (`SpringArmComponent.TargetArmLength` _cameraboom))
  (set `self.Sum` (+ (`self.Sum`) _cameratickstep))
  (set `SpringArmComponent.TargetArmLength` (select `bool` (`self.SlideUp`) :`false` (- _targetarmlength _cameratickstep) :`true` (+ _cameratickstep _targetarmlength)) _cameraboom)
  (if (== (`self.Sum`) (`self.CameraStep`))
    (set `self.Sum` 0.0)
    (set `self.SlideDone` true)
    (`KismetSystemLibrary.K2_ClearAndInvalidateTimerHandle` (`self.TimerSlide`))))

(fn `CameraZoom`
  (params (A :type "Float (double-precision)"))
  (bind _cameraboom (`self.CameraBoom`))
  (if (> A 0.0)
    (set `SpringArmComponent.TargetArmLength` (- (`SpringArmComponent.TargetArmLength` _cameraboom) (`self.CameraStep`)) _cameraboom)
    (elif (< A 0.0)
      (set `SpringArmComponent.TargetArmLength` (+ (`self.CameraStep`) (`SpringArmComponent.TargetArmLength` _cameraboom)) _cameraboom))))

(fn `ChangeWeaponWidgetName`
  (bind _foundwidgets (`WidgetBlueprintLibrary.GetAllWidgetsOfClass` "/Game/Widget/Inventory/WeaponSlot.WeaponSlot_C" false))
  (for _array_element _foundwidgets
    (bind _returnvalue (`self.GetCurrentWeapon`))
    (bind _returnvalue_2 (`DefaultWeapon.GetWeaponSetting` _returnvalue))
    (if (== (`/Game/Widget/Inventory/WeaponSlot.IdNameWeapon` _array_element) (`.WeaponName` (break `WeaponInfo` _returnvalue_2)))
      (set `/Game/Widget/Inventory/WeaponSlot.IdNameWeapon` (`.ItemName` (break `WeaponSlot` (`/Game/Blueprint/Characters/PickUpWeapons/PickupActor_Weapon.WeaponSlotByDefault` (`self.PickupedWeapon`)))) _array_element))))

(fn `CharDead`
  (`PrimitiveComponent.SetCollisionResponseToChannel` (`self.CapsuleComponent`) "ECC_Pawn" "ECR_Ignore")
  (`PrimitiveComponent.SetCollisionResponseToChannel` (`self.Mesh`) "ECC_Pawn" "ECR_Ignore")
  (bind _returnvalue (`|CreateWidget` "/Game/Widget/BPW_DeathWidget.BPW_DeathWidget_C"))
  (`UserWidget.AddToViewport` _returnvalue 0)
  (set `PlayerController.bShowMouseCursor` true (`GameplayStatics.GetPlayerController` 0)))

(fn `DisablePawnMovement`
  (set `self.InputBlock` true)
  (`SceneComponent.SetVisibility` (`self.CursorToWorld`) false false))

(fn `EnablePawnMovement`
  (set `self.InputBlock` false)
  (`SceneComponent.SetVisibility` (`self.CursorToWorld`) true false))

(fn `OnRep_BP Spawn Loot`)

(fn `SeeThroughBoxes`
  (bind _outhits (`KismetSystemLibrary.LineTraceMulti` :`Start` (`SceneComponent.K2_GetComponentLocation` (`self.TopDownCameraComponent`)) :`End` (`SceneComponent.K2_GetComponentLocation` (`self.CursorToWorld`)) :`TraceChannel` "TraceTypeQuery4" :`DrawTime` 2.0))
  (for _array_element _outhits
    (bind (_bblockinghit _binitialoverlap _time _distance _location _impactpoint _normal _impactnormal _physmat _hitactor _hitcomponent) (`GameplayStatics.BreakHitResult` _array_element))
    (if (not (!= (`KismetStringLibrary.FindSubstring` (`KismetSystemLibrary.GetDisplayName` _hitactor) "SM_L" false false 0) 0))
      (`PrimitiveComponent.SetMaterial` _hitcomponent 0 "/Game/All_added_content/MI_RoofSingles_Inst.MI_RoofSingles_Inst"))))

(fn `UserConstructionScript`
  (bind _cameraboom (`self.CameraBoom`))
  (set `SpringArmComponent.TargetArmLength` (`self.Hieght`) _cameraboom)
  (`SceneComponent.K2_SetRelativeRotation` _cameraboom (`self.Rotation`) false false)
  (set `SpringArmComponent.bEnableCameraLag` (`self.Flow`) _cameraboom)
  (set `SpringArmComponent.CameraLagSpeed` (`self.CoefSmooth`) _cameraboom))
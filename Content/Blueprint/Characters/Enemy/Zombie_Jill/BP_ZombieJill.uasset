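; Zombie Jill enemy character with physics-driven hit reactions, floating damage numbers and a cinematic death.
; Point damage lowers the health component and simulates bodies below a bone under physical animation, with a timer stopping simulation.
; Death unpossesses the controller and plays a random montage, then ragdolls and drops a random item.
; When the last Zombie Jill dies, a glory camera spawns at a random camera component, slowing time and disabling player movement.
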(event `self.ReceivePointDamage`
  (params (Damage :type "Float (single-precision)") (DamageType :type "DamageType Object Reference") (HitLocation :type "Vector Structure") (HitNormal :type "Vector Structure") (HitComponent :type "PrimitiveComponent Object Reference") (BoneName :type Name) (ShotFromDirection :type "Vector Structure") (InstigatedBy :type "Controller Object Reference") (DamageCauser :type "Actor Object Reference") (HitInfo :type "HitResult Structure (by ref)"))
  (`SkeletalMeshComponent.SetAllBodiesBelowSimulatePhysics` (`self.Mesh`) (`self.Body Name`) true false)
  (if (not (`self.bIsDead`))
    (bind _returnvalue (`KismetSystemLibrary.K2_SetTimerDelegate` (delegate `PhysicsStop`) 5.0))
    (set `self.BodyToDefaultTimer` _returnvalue)
    (bind _returnvalue_2 (`HeathComponent.GetCurrentHealth` (`self.Heath`)))
    (if (> _returnvalue_2 1.0)
      (`HeathComponent.ChangeCurrentHealth` (`self.Heath`) (* -1 Damage)))))

(event `PhysicsStop`
  (`SkeletalMeshComponent.SetAllBodiesBelowSimulatePhysics` (`self.Mesh`) (`self.Body Name`) false true))

(event `self.ReceiveAnyDamage`
  (params (Damage :type "Float (single-precision)") (DamageType :type "DamageType Object Reference") (InstigatedBy :type "Controller Object Reference") (DamageCauser :type "Actor Object Reference")))

(event `self.Heath.OnHeathChange`
  (params (Health :type "Float (single-precision)") (Damage :type "Float (single-precision)"))
  (bind _returnvalue (`|SpawnActorFromClass` "/Game/Blueprint/Characters/CanTakeDamageObjects/DisplayDamageActor.DisplayDamageActor_C" (`KismetMathLibrary.MakeTransform` (+ (`self.K2_GetActorLocation`) (+ (`self.LocalPointSpawnHealthNumber`) (`KismetMathLibrary.MakeVector` (`KismetMathLibrary.RandomFloatInRange` 0.0 40.0) (`KismetMathLibrary.RandomFloatInRange` 0.0 40.0))))) "Undefined" "OverrideRootScale" null null))
  (`/Game/Blueprint/Characters/CanTakeDamageObjects/DisplayDamageActor.InitActor` _returnvalue Damage Health))

(event `self.ReceiveBeginPlay`
  (bind _physicalanimation (`self.PhysicalAnimation`))
  (add `HeathComponent.OnDead` (`self.Heath`) (delegate `OnDeadHealth`))
  (`PhysicalAnimationComponent.SetSkeletalMeshComponent` _physicalanimation (`self.Mesh`))
  (`PhysicalAnimationComponent.ApplyPhysicalAnimationSettingsBelow` _physicalanimation (`self.Body Name`) (make `PhysicalAnimationData` false 2000.0 20.0 2000.0 20.0) false))

(event `OnDeadHealth`
  (bind _deathmontages (`self.DeathMontages`))
  (bind _returnvalue (`KismetArrayLibrary.Array_Length` _deathmontages))
  (bind _output (`|GetArrayItem` _deathmontages (`KismetMathLibrary.RandomIntegerInRange` 0 (- _returnvalue 1))))
  (`self.DeadFunc`)
  (if (> _returnvalue 0)
    (`PrimitiveComponent.SetCollisionEnabled` (`self.CapsuleComponent`) "NoCollision")
    (bind _returnvalue_2 (`AnimSequenceBase.GetPlayLength` _output))
    (`|PlayMontage` (`self.Mesh`) _output
      (:`then`
        (bind _returnvalue_3 (* _returnvalue_2 0.7))
        (bind _returnvalue_4 (`KismetSystemLibrary.K2_SetTimerDelegate` (delegate `RagDoll`) _returnvalue_3))
        (`self.GloryCamera` _returnvalue_3)))))

(event `RagDoll`
  (bind _physicalanimation (`self.PhysicalAnimation`))
  (`PrimitiveComponent.SetCollisionEnabled` (`self.Mesh`) "PhysicsOnly")
  (`PrimitiveComponent.SetCollisionResponseToChannel` (`self.Mesh`) "ECC_PhysicsBody" "ECR_Ignore")
  (`PrimitiveComponent.SetSimulatePhysics` (`self.Mesh`) true)
  (`DropItemComponent.DropRandomItem` (`self.DropItemComponent`) (0.0 0.0 0.0) 50 5 0 0)
  (`PhysicalAnimationComponent.SetSkeletalMeshComponent` _physicalanimation null)
  (`ActorComponent.Deactivate` _physicalanimation)
  (`KismetSystemLibrary.K2_ClearAndInvalidateTimerHandle` (stale `OnDeadHealth` _returnvalue_4)))

(event `self.ReceiveTick`
  (params (DeltaSeconds :type "Float (single-precision)")))

(fn `DeadFunc`
  (`self.SetStateAttack` false)
  (`self.SetStateMovement` false)
  (`Controller.UnPossess` (`self.GetController`))
  (`self.SetLifeSpan` 10.0)
  (set `self.bIsDead` true)
  (`KismetSystemLibrary.K2_ClearAndInvalidateTimerHandle` (`self.BodyToDefaultTimer`)))

(fn `GloryCamera`
  (params (AnimationTime :type "Float (double-precision)"))
  (bind _returnvalue (`self.K2_GetComponentsByClass` self "/Script/Engine.CameraComponent"))
  (bind _outactors (`GameplayStatics.GetAllActorsOfClass` "BP_ZombieJill_C"))
  (bind _returnvalue_2 (`KismetArrayLibrary.Array_Length` _outactors))
  (`KismetSystemLibrary.PrintString` (`KismetStringLibrary.Conv_IntToString` _returnvalue_2))
  (if (<= _returnvalue_2 1)
    (bind _returnvalue_3 (`|SpawnActorFromClass` "/Script/Engine.CameraActor" (`SceneComponent.K2_GetComponentToWorld` (`|GetArrayItem` _returnvalue (`KismetMathLibrary.RandomIntegerInRange` 0 (- (`KismetArrayLibrary.Array_Length` _returnvalue) 1)))) "Undefined" "OverrideRootScale" null null))
    (bind _output_get (set `self.GloryCameraActor` _returnvalue_3))
    (`PlayerController.SetViewTargetWithBlend` (`GameplayStatics.GetPlayerController` 0) _output_get 0.0 "VTBlend_Linear" 0.0 false)
    (bind _returnvalue_4 (`KismetSystemLibrary.K2_SetTimerDelegate` (`|CreateDelegate` :!event `SetToDefaultCamera`) AnimationTime))
    (set `self.GloryCameraTimer` _returnvalue_4)
    (`GameplayStatics.SetGlobalTimeDilation` 0.3)
    (bind _asbp_character (cast `/Game/Blueprint/Characters/BP_Character` (`GameplayStatics.GetPlayerPawn` 0)))
    (`SceneComponent.SetVisibility` (`HomeWork22Character.CursorToWorld` _asbp_character) false false)
    (`/Game/Blueprint/Characters/BP_Character.DisablePawnMovement` _asbp_character)))

(fn `SetStateAttack`
  (params (CanAttack :type Boolean))
  (set `self.bCanAttack` CanAttack))

(fn `SetStateMovement`
  (params (`Can Move` :type Boolean))
  (set `self.bCanMove` `Can Move`))

(fn `SetToDefaultCamera`
  (bind _glorycameraactor (`self.GloryCameraActor`))
  (`/Engine/EditorBlueprintResources/StandardMacros.IsValid` _glorycameraactor
    (:`Is Valid`
      (`self.K2_DestroyActor` _glorycameraactor))
    (:`Is Not Valid`
      _))
  (`KismetSystemLibrary.K2_ClearAndInvalidateTimerHandle` (`self.GloryCameraTimer`))
  (`GameplayStatics.SetGlobalTimeDilation` 1.0)
  (bind _asbp_character (cast `/Game/Blueprint/Characters/BP_Character` (`GameplayStatics.GetPlayerPawn` 0)))
  (`SceneComponent.SetVisibility` (`HomeWork22Character.CursorToWorld` _asbp_character) true false)
  (`/Game/Blueprint/Characters/BP_Character.EnablePawnMovement` _asbp_character))

(fn `UserConstructionScript`)
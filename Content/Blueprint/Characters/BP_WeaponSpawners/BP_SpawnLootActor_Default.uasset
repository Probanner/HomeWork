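; Loot case actor that scatters random item drops and then destroys itself, dropping more items at higher rarity.
; On BeginPlay it can roll a random case that sets rarity, mesh, glowing particle color and a custom depth stencil per rarity.
; Its collision sphere notifies BP_Character on overlap start and end.
; SpawnPickupActor drops items through DropItemComponent, randomly yawing a spawn arrow to aim each one.
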(event `self.ReceiveBeginPlay`
  (if (`self.RandomCase`)
    (bind _returnvalue (`self.GetRandomCase`))
    (bind (_skeletalmesh _staticmesh _lootrariness _lootcolor) (break `LootCase` _returnvalue))
    (set `self.Rariness` _lootrariness)
    (`FXSystemComponent.SetColorParameter` (`self.ParticleFx`) "ScaleColor" (* _lootcolor 5.0))
    (`StaticMeshComponent.SetStaticMesh` (`self.StaticMeshComp`) _staticmesh)
    (bind _returnvalue_2 (`PrimitiveComponent.CreateDynamicMaterialInstance` (`self.ParticleFx`) 0 null "None"))
    (`MaterialInstanceDynamic.SetScalarParameterValue` _returnvalue_2 "Emission" 5.0)
    (`PrimitiveComponent.SetCustomDepthStencilValue` (`self.StaticMeshComp`) (select `ERariness` (`self.Rariness`) :`Common_Type` 1 :`Rare_Type` 2 :`Epic_Type` 3 :`Legendary_Type` 4))))

(event `Delay1`
  (`KismetSystemLibrary.Delay` 5.0))

(event `self.ReceiveTick`
  (params (DeltaSeconds :type "Float (single-precision)")))

(event `self.CollisionSphere.OnComponentBeginOverlap`
  (params (OverlappedComponent :type "PrimitiveComponent Object Reference") (OtherActor :type "Actor Object Reference") (OtherComp :type "PrimitiveComponent Object Reference") (OtherBodyIndex :type Integer) (bFromSweep :type Boolean) (SweepResult :type "HitResult Structure (by ref)"))
  (bind _asbp_character (cast `/Game/Blueprint/Characters/BP_Character` OtherActor))
  (`/Game/Blueprint/Characters/BP_Character.LootCaseStartOverlap` _asbp_character self))

(event `self.CollisionSphere.OnComponentEndOverlap`
  (params (OverlappedComponent :type "PrimitiveComponent Object Reference") (OtherActor :type "Actor Object Reference") (OtherComp :type "PrimitiveComponent Object Reference") (OtherBodyIndex :type Integer))
  (bind _asbp_character (cast `/Game/Blueprint/Characters/BP_Character` OtherActor))
  (`/Game/Blueprint/Characters/BP_Character.LootCaseOverlapEnd` _asbp_character))

(fn `BP_SpawnLootActor_Default_AutoGenFunc`)

(fn `Spawn Pickup Actor`
  (`self.SpawnItems` (select `ERariness` (`self.Rariness`) :`Rare_Type` 1 :`Epic_Type` 2 :`Legendary_Type` 3))
  (`self.K2_DestroyActor`))

(fn `SpawnItems`
  (params (CountOfItems :type Integer))
  (bind _arrowspawncomp (`self.ArrowSpawnComp`))
  (bind (_relativerotation_roll _relativerotation_pitch _relativerotation_yaw) (`KismetMathLibrary.BreakRotator` (`SceneComponent.RelativeRotation` _arrowspawncomp)))
  (for _ (range (+ (+ CountOfItems 1) 1))
    (`SceneComponent.K2_SetRelativeRotation` _arrowspawncomp (`KismetMathLibrary.MakeRotator` _relativerotation_roll _relativerotation_pitch (+ _relativerotation_yaw (* (`KismetMathLibrary.RandomIntegerInRange` -10 10) 30.0))) false false)
    (`DropItemComponent.DropRandomItem` (`self.DropItemComponent`) (`SceneComponent.GetForwardVector` (`self.ArrowSpawnComp`)))
    (`self.Delay1`)))

(fn `UserConstructionScript`)
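; BP_Cube is an actor with a cube mesh that turns partly see-through while the mouse cursor hovers over it.
; On BeginPlay it creates a dynamic material instance from Translucent_Material and applies it to the cube.
; The cube's cursor-over events lower the material's Opacity parameter on hover and restore it to fully opaque when the cursor leaves.
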(event `self.ReceiveBeginPlay`
  (bind _returnvalue (`KismetMaterialLibrary.CreateDynamicMaterialInstance` "/Game/Enviroment/Materials/Translucent_Material.Translucent_Material"))
  (set `self.DynamicMat` _returnvalue)
  (`PrimitiveComponent.SetMaterial` (`self.Cube`) 0 (`self.DynamicMat`)))

(event `self.Cube.OnBeginCursorOver`
  (params (TouchedComponent :type "PrimitiveComponent Object Reference"))
  (`MaterialInstanceDynamic.SetScalarParameterValue` (`self.DynamicMat`) "Opacity" 0.6))

(event `self.Cube.OnEndCursorOver`
  (params (TouchedComponent :type "PrimitiveComponent Object Reference"))
  (`MaterialInstanceDynamic.SetScalarParameterValue` (`self.DynamicMat`) "Opacity" 1.0))

(fn `UserConstructionScript`)
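; Cabin level actor with a furnace sound, a door that swings open when the player approaches, and the Necronomicon cutscene.
; Touching the book's trigger once freezes the player, fires a dispatcher, cuts to book and gate cameras, then restores view and control.
; Looping timers rotate door and gates and burn away the book through Material Parameter Collection scalars.
; Roof-transparency helpers exist but are unwired; only the original-material caching runs.
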(event `self.ReceiveTick`
  (params (DeltaSeconds :type "Float (single-precision)")))

(event `self.ReceiveBeginPlay`
  (`self.SaveOriginal`)
  (`GameplayStatics.PlaySoundAtLocation` "/Game/LogCabin/Audio/SC_Furnace.SC_Furnace" (`SceneComponent.K2_GetComponentLocation` (`self.SM_Fire_Flames2`)) (struct) 0.5 1.0 0.0 null null null)
  (bind _returnvalue (`KismetMaterialLibrary.GetScalarParameterValue` "/Game/All_added_content/Parameter_Collection_Nerconomicon.Parameter_Collection_Nerconomicon" "FadeParameter"))
  (bind _output_get (set `self.OpacityMaskSum` _returnvalue))
  (set `self.OpacityMaskSum_Temp` _output_get)
  (bind _returnvalue_2 (`KismetMaterialLibrary.GetScalarParameterValue` "/Game/All_added_content/Parameter_Collection_Nerconomicon.Parameter_Collection_Nerconomicon" "EmissiveParam"))
  (bind _output_get_2 (set `self.EmissiveValueSum` _returnvalue_2))
  (set `self.EmissiveValueSum_Temp` _output_get_2))

(event `self.InHouseBox.OnComponentBeginOverlap`
  (params (OverlappedComponent :type "PrimitiveComponent Object Reference") (OtherActor :type "Actor Object Reference") (OtherComp :type "PrimitiveComponent Object Reference") (OtherBodyIndex :type Integer) (bFromSweep :type Boolean) (SweepResult :type "HitResult Structure (by ref)")))

(event `self.OutHouseBox.OnComponentBeginOverlap`
  (params (OverlappedComponent :type "PrimitiveComponent Object Reference") (OtherActor :type "Actor Object Reference") (OtherComp :type "PrimitiveComponent Object Reference") (OtherBodyIndex :type Integer) (bFromSweep :type Boolean) (SweepResult :type "HitResult Structure (by ref)")))

(event `self.InHouseDoorOpenBox.OnComponentBeginOverlap`
  (params (OverlappedComponent :type "PrimitiveComponent Object Reference") (OtherActor :type "Actor Object Reference") (OtherComp :type "PrimitiveComponent Object Reference") (OtherBodyIndex :type Integer) (bFromSweep :type Boolean) (SweepResult :type "HitResult Structure (by ref)"))
  (cast `/Game/Blueprint/Characters/BP_Character` OtherActor)
  (if (not (`self.DoorIsOpen`))
    (`GameplayStatics.PlaySoundAtLocation` "/Game/Blueprint/Sound/DoorOpenSound.DoorOpenSound" (`SceneComponent.K2_GetComponentLocation` (`self.SM_Door_Door`)) (struct) 0.5 1.0 0.0 null null null)
    (bind _returnvalue (`KismetSystemLibrary.K2_SetTimer` null "DoorOpen" (`self.TimerTick`) true))
    (set `self.TimerHandle` _returnvalue)
    (set `self.DoorIsOpen` true)))

(event `self.NecronomiconBox.OnComponentBeginOverlap`
  (params (OverlappedComponent :type "PrimitiveComponent Object Reference") (OtherActor :type "Actor Object Reference") (OtherComp :type "PrimitiveComponent Object Reference") (OtherBodyIndex :type Integer) (bFromSweep :type Boolean) (SweepResult :type "HitResult Structure (by ref)"))
  (bind _asbp_character (cast `/Game/Blueprint/Characters/BP_Character` OtherActor))
  (if (not (`self.bNecronomicon_Activated`))
    (set `self.bNecronomicon_Activated` true)
    (`/Game/Blueprint/Characters/BP_Character.DisablePawnMovement` _asbp_character)
    (`self.NecronomiconDispatcher`)
    (`GameplayStatics.PlaySound2D` "/Game/Blueprint/Sound/Thunder.Thunder" 0.5 1.0 0.0 null null)
    (bind _returnvalue (`KismetSystemLibrary.K2_SetTimer` null "BookDisappear" 0.05 true))
    (set `self.NecroTimerHandle` _returnvalue)
    (bind _returnvalue_2 (`self.CameraChange` (`SceneComponent.GetRelativeTransform` (`self.CameraNecro`))))
    (`GameplayStatics.PlaySoundAtLocation` "/Game/Blueprint/Sound/paperburn1_Cue.paperburn1_Cue" (`SceneComponent.K2_GetComponentLocation` (`self.book`)) (struct) 1.0 1.0 0.7 null null null)
    (`KismetSystemLibrary.Delay` 6.0)
    (`GameplayStatics.PlaySoundAtLocation` "/Game/Blueprint/Sound/gate2.gate2" (`SceneComponent.K2_GetComponentLocation` (`self.SM_Fence_Pole2`)) (struct) 0.5 1.0 0.0 null null null)
    (bind _returnvalue_3 (`self.CameraChange` (`SceneComponent.GetRelativeTransform` (`self.CameraGate`))))
    (bind _returnvalue_4 (`KismetSystemLibrary.K2_SetTimer` null "OpenGates" 0.01 true))
    (set `self.GatesTimerHandle` _returnvalue_4)
    (`KismetSystemLibrary.Delay` 5.0)
    (`PlayerController.SetViewTargetWithBlend` (`GameplayStatics.GetPlayerController` 0) (`GameplayStatics.GetPlayerCharacter` 0) 1.0 "VTBlend_Linear" 0.0 true)
    (`ActorComponent.K2_DestroyComponent` _returnvalue_2)
    (`ActorComponent.K2_DestroyComponent` _returnvalue_3)
    (`KismetSystemLibrary.K2_ClearAndInvalidateTimerHandle` (`self.GatesTimerHandle`))
    (`KismetSystemLibrary.K2_ClearAndInvalidateTimerHandle` (`self.NecroTimerHandle`))
    (`/Game/Blueprint/Characters/BP_Character.EnablePawnMovement` _asbp_character)))

(fn `BookDisappear`
  (locals (OpacityStep :type "Float (double-precision)" :default 0.01))
  (bind _opacitystep (`local.OpacityStep`))
  (bind _book (`self.book`))
  (bind _yup (`self.YUp`))
  (bind _returnvalue (- (`self.OpacitySum`) _opacitystep))
  (if (<= (`self.OpacityMaskSum_Temp`) 0.0)
    (`KismetSystemLibrary.K2_ClearAndInvalidateTimerHandle` (`self.NecroTimerHandle`))
    (`ActorComponent.K2_DestroyComponent` (`self.NecronomiconParticleSystem`))
    (else
      (`KismetMaterialLibrary.SetScalarParameterValue` "/Game/All_added_content/Parameter_Collection_Nerconomicon.Parameter_Collection_Nerconomicon" "Opacity" _returnvalue)
      (set `self.OpacitySum` _returnvalue)
      (bind _output_get (set `self.OpacityMaskSum_Temp` (- (`self.OpacityMaskSum_Temp`) (- (`self.OpacityMaskSum`) (`KismetMathLibrary.Lerp` (`self.OpacityMaskSum`) 0.0 _opacitystep)))))
      (`KismetMaterialLibrary.SetScalarParameterValue` "/Game/All_added_content/Parameter_Collection_Nerconomicon.Parameter_Collection_Nerconomicon" "FadeParameter" _output_get)
      (bind _output_get_2 (set `self.f_Emissive` (`KismetMathLibrary.Lerp` (`self.f_Emissive`) 5.0 _opacitystep)))
      (`KismetMaterialLibrary.SetScalarParameterValue` "/Game/All_added_content/Parameter_Collection_Nerconomicon.Parameter_Collection_Nerconomicon" "EmissiveParam" _output_get_2)
      (if (!= _output_get_2 0.0)
        (`KismetMaterialLibrary.SetScalarParameterValue` "/Game/All_added_content/Parameter_Collection_Nerconomicon.Parameter_Collection_Nerconomicon" "LerpFire" (- _output_get_2 2.0)))
      (`SceneComponent.K2_AddLocalOffset` _book (`KismetMathLibrary.MakeVector` 0.0 _yup) false false)
      (`SceneComponent.K2_AddRelativeRotation` _book (`KismetMathLibrary.MakeRotator` (`KismetMathLibrary.Abs` _yup)) false false)
      (if (not (`self.b_ParticeFire`))
        (`GameplayStatics.SpawnEmitterAttached` "/Game/Fx_Effect/Particles/P_FireBurn.P_FireBurn" (`self.book`) "None" (0.0 0.0 0.0) (struct :`Pitch` 120.0) (0.1 0.1 0.1))
        (`GameplayStatics.PlaySound2D` "/Game/Blueprint/Sound/EvilLaugh.EvilLaugh" 1.0 1.0 0.0 null null)
        (set `self.b_ParticeFire` true)))))

(fn `CameraChange`
  (params (RelativeTransform :type "Transform Structure"))
  (returns (ReturnValue :type "ChildActorComponent Object Reference"))
  (bind _returnvalue (`AddComponent|NODE_AddChildActorComponent-0` :`RelativeTransform` RelativeTransform))
  (`PlayerController.SetViewTargetWithBlend` (`GameplayStatics.GetPlayerController` 0) (`ChildActorComponent.ChildActor` _returnvalue) (`self.CameraSwitchTime`) "VTBlend_Linear" 0.0 false)
  (return _returnvalue))

(fn `DoorOpen`
  (locals (RotateDoorStep :type "Float (double-precision)" :default -1.0))
  (bind _output_get (set `self.Sum` (+ (`self.Sum`) (`local.RotateDoorStep`))))
  (if (<= _output_get -110.0)
    (`KismetSystemLibrary.K2_ClearAndInvalidateTimerHandle` (`self.TimerHandle`))
    (else
      (`SceneComponent.K2_SetRelativeRotation` (`self.SM_Door_Door`) (`KismetMathLibrary.MakeRotator` 0.0 0.0 _output_get) false false))))

(fn `OpenGates`
  (locals (GatesOpenStep :type "Float (double-precision)" :default 0.2))
  (bind _gatesopenstep (`local.GatesOpenStep`))
  (if (>= (`self.GatesOpenHight`) 90.0)
    (`KismetSystemLibrary.K2_ClearAndInvalidateTimerHandle` (`self.GatesTimerHandle`))
    (else
      (`SceneComponent.K2_AddRelativeRotation` (`self.SM_Door_Door1`) (`KismetMathLibrary.MakeRotator` 0.0 0.0 (* -1 _gatesopenstep)) false false)
      (`SceneComponent.K2_AddRelativeRotation` (`self.SM_Door_Door2`) (`KismetMathLibrary.MakeRotator` 0.0 0.0 _gatesopenstep) false false)
      (set `self.GatesOpenHight` (+ (`self.GatesOpenHight`) _gatesopenstep)))))

(fn `SaveOriginal`
  (set `self.SM_Logcabin_Roof_Beams_original` (`PrimitiveComponent.GetMaterial` (`self.SM_Logcabin_Roof_Beams_02`) 0))
  (set `self.SM_Logcabin_Logs_02_original` (`PrimitiveComponent.GetMaterial` (`self.SM_Logcabin_Logs_02`) 0))
  (set `self.SM_Logcabin_Beams_original` (`PrimitiveComponent.GetMaterial` (`self.SM_Logcabin_Beams_01`) 0))
  (set `self.SM_Logcabin_RoofShingles_original` (`PrimitiveComponent.GetMaterial` (`self.SM_Logcabin_RoofShingles`) 0))
  (set `self.SM_LC_Addon_Ceiling_original` (`PrimitiveComponent.GetMaterial` (`self.SM_LC_Addon_Ceiling`) 0))
  (set `self.SM_Logcabin_Logs_01_original` (`PrimitiveComponent.GetMaterial` (`self.SM_Logcabin_Logs_01`) 0))
  (set `self.SM_Logcabin_RoofShingles001_original` (`PrimitiveComponent.GetMaterial` (`self.SM_Logcabin_RoofShingles001`) 0))
  (set `self.SM_Logcabin_Beams_original1` (`PrimitiveComponent.GetMaterial` (`self.SM_Logcabin_Beams`) 0))
  (set `self.SM_Logcabin_Roof_Porch_original` (`PrimitiveComponent.GetMaterial` (`self.SM_Logcabin_Roof_Porch`) 0))
  (set `self.SM_Logcabin_Porch_Beams_original` (`PrimitiveComponent.GetMaterial` (`self.SM_Logcabin_Porch_Beams`) 0)))

(fn `SetSellingInvisible`
  (`PrimitiveComponent.SetMaterial` (`self.SM_Logcabin_Roof_Beams_02`) 0 "/Game/All_added_content/MI_TransparentRoof.MI_TransparentRoof")
  (`PrimitiveComponent.SetMaterial` (`self.SM_Logcabin_Logs_02`) 0 "/Game/All_added_content/MI_TransparentRoof.MI_TransparentRoof")
  (`PrimitiveComponent.SetMaterial` (`self.SM_Logcabin_Beams_01`) 0 "/Game/All_added_content/MI_TransparentRoof.MI_TransparentRoof")
  (`PrimitiveComponent.SetMaterial` (`self.SM_Logcabin_RoofShingles`) 0 "/Game/All_added_content/MI_TransparentRoof.MI_TransparentRoof")
  (`PrimitiveComponent.SetMaterial` (`self.SM_LC_Addon_Ceiling`) 0 "/Game/All_added_content/MI_TransparentRoof.MI_TransparentRoof")
  (`PrimitiveComponent.SetMaterial` (`self.SM_Logcabin_Logs_01`) 0 "/Game/All_added_content/MI_TransparentRoof.MI_TransparentRoof")
  (`PrimitiveComponent.SetMaterial` (`self.SM_Logcabin_RoofShingles001`) 0 "/Game/All_added_content/MI_TransparentRoof.MI_TransparentRoof")
  (`PrimitiveComponent.SetMaterial` (`self.SM_Logcabin_Beams`) 0 "/Game/All_added_content/MI_TransparentRoof.MI_TransparentRoof")
  (`PrimitiveComponent.SetMaterial` (`self.SM_Logcabin_Roof_Porch`) 0 "/Game/All_added_content/MI_TransparentRoof.MI_TransparentRoof")
  (`PrimitiveComponent.SetMaterial` (`self.SM_Logcabin_Porch_Beams`) 0 "/Game/All_added_content/MI_TransparentRoof.MI_TransparentRoof")
  (`PrimitiveComponent.SetMaterial` (`self.SM_Logcabin_Beams_02`) 0 "/Game/All_added_content/MI_TransparentRoof.MI_TransparentRoof"))

(fn `SetSellingToNormal`
  (bind _sm_logcabin_porch_beams_original (`self.SM_Logcabin_Porch_Beams_original`))
  (`PrimitiveComponent.SetMaterial` (`self.SM_Logcabin_Roof_Beams_02`) 0 (`self.SM_Logcabin_Roof_Beams_original`))
  (`PrimitiveComponent.SetMaterial` (`self.SM_Logcabin_Logs_02`) 0 (`self.SM_Logcabin_Logs_02_original`))
  (`PrimitiveComponent.SetMaterial` (`self.SM_Logcabin_Beams_01`) 0 (`self.SM_Logcabin_Beams_original`))
  (`PrimitiveComponent.SetMaterial` (`self.SM_Logcabin_RoofShingles`) 0 (`self.SM_Logcabin_RoofShingles_original`))
  (`PrimitiveComponent.SetMaterial` (`self.SM_LC_Addon_Ceiling`) 0 (`self.SM_LC_Addon_Ceiling_original`))
  (`PrimitiveComponent.SetMaterial` (`self.SM_Logcabin_Logs_01`) 0 (`self.SM_Logcabin_Logs_01_original`))
  (`PrimitiveComponent.SetMaterial` (`self.SM_Logcabin_RoofShingles001`) 0 (`self.SM_Logcabin_RoofShingles001_original`))
  (`PrimitiveComponent.SetMaterial` (`self.SM_Logcabin_Beams`) 0 (`self.SM_Logcabin_Beams_original1`))
  (`PrimitiveComponent.SetMaterial` (`self.SM_Logcabin_Roof_Porch`) 0 (`self.SM_Logcabin_Roof_Porch_original`))
  (`PrimitiveComponent.SetMaterial` (`self.SM_Logcabin_Porch_Beams`) 0 _sm_logcabin_porch_beams_original)
  (`PrimitiveComponent.SetMaterial` (`self.SM_Logcabin_Beams`) 0 _sm_logcabin_porch_beams_original)
  (`PrimitiveComponent.SetMaterial` (`self.SM_Logcabin_Beams_02`) 0 _sm_logcabin_porch_beams_original))

(fn `UserConstructionScript`)
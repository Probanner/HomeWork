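; BP_EnviromentStructure is an environment structure actor with a health component and a list of effects.
; Each tick it prints every effect's name and the current health to screen as debug output.
; AvailableForEffects logs a message and always returns false.
; On death it spawns a fire explosion emitter at its scene component's location and destroys itself, while the damage and overlap events are empty.
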(event `self.ReceiveBeginPlay`)

(event `self.ReceiveTick`
  (params (DeltaSeconds :type "Float (single-precision)"))
  (for _array_element (`self.Effects`)
    (`KismetSystemLibrary.PrintString` (`KismetSystemLibrary.GetDisplayName` _array_element) true true (struct :`G` 0.66 :`B` 1.0 :`A` 1.0) 0.0)
    (bind _returnvalue (`HeathComponent.GetCurrentHealth` (`self.Heath`)))
    (`KismetSystemLibrary.PrintString` (`KismetStringLibrary.Concat_StrStr` "Current Health = " (`KismetStringLibrary.Conv_DoubleToString` _returnvalue)) true true (struct :`G` 0.66 :`B` 1.0 :`A` 1.0) 0.0)))

(event `self.AvailableForEffectsBP`)

(event `self.ReceiveRadialDamage`
  (params (DamageReceived :type "Float (single-precision)") (DamageType :type "DamageType Object Reference") (Origin :type "Vector Structure") (HitInfo :type "HitResult Structure (by ref)") (InstigatedBy :type "Controller Object Reference") (DamageCauser :type "Actor Object Reference")))

(event `self.ReceiveAnyDamage`
  (params (Damage :type "Float (single-precision)") (DamageType :type "DamageType Object Reference") (InstigatedBy :type "Controller Object Reference") (DamageCauser :type "Actor Object Reference")))

(fn `AvailableForEffects`
  (returns (ReturnValue :type Boolean))
  (`KismetSystemLibrary.PrintString` "Available for Effects")
  (return false))

(fn `OnDeadIvent`
  (`GameplayStatics.SpawnEmitterAtLocation` "/Game/M5VFXVOL2/Particles/Explosion/Fire_Exp_00.Fire_Exp_00" (`SceneComponent.K2_GetComponentLocation` (`self.SceneComponent`)))
  (`self.K2_DestroyActor`))

(fn `UserConstructionScript`)